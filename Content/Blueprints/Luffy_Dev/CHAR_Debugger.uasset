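; Debug character that flies through the level, with an on-screen HUD for inspecting the world.
; Input moves it by teleporting offsets along control-yaw axes, with mouse-wheel speed scaling.
; Keys toggle gravity with collision and capsule physics, respawn at the start point while setting world origin, and show or hide HUD readouts.
; Tick updates enabled readouts: position, control rotation, and the actor name hit by a camera line trace.
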(event EventBeginPlay
  ;[0.5308 1 0.04161] Initalization
  (Input|EnableInput (Game|GetPlayerController 0))
  (Variables|respawn|SetspawnedVector (Transformation|GetActorLocation))
  (bind _returnvalue (UserInterface|CreateWidget "/Game/Blueprints/Luffy_Dev/HUD_Debugger.HUD_Debugger_C" (Game|GetPlayerController 0)))
  (bind _output_get (Variables|UMG|SetHUD_Info _returnvalue))
  (UserInterface|Viewport|AddtoViewport _output_get 0))

(event EventTick
  (params (DeltaSeconds :type Float%20%28single-precision%29))
  ;[0.3736 1 0.9602] Tick
  (Utilities|FlowControl|Sequence
    (:then_0
      (if (Variables|Flags|GetposFlag)
        (CallFunction|SetNewPosInfo)))
    (:then_1
      (if (Variables|Flags|GettraceFlag)
        (CallFunction|TracetoObject)))))

(event Input|AxisEvents|InputAxisKeyboardForward
  (params (AxisValue :type Float%20%28single-precision%29))
  ;[1 0.09121 0] Forward/Back Input
  (bind _forwardvector (CallFunction|GetForwardVector))
  (Transformation|AddActorWorldOffset (* (* (* (* _forwardvector AxisValue) (Variables|MoveRate|GetforRate)) (Utilities|Time|GetWorldDeltaSeconds)) (Variables|MoveRate|GetmoveMulitplier)) false true))

(event Input|AxisEvents|InputAxisKeyboardRight
  (params (AxisValue :type Float%20%28single-precision%29))
  ;[0.0514 0.06834 1] Left/Right Input
  (bind _rightvector (CallFunction|GetRightVector))
  (Transformation|AddActorWorldOffset (* (* (* (* _rightvector AxisValue) (Variables|MoveRate|GetstrafeRate)) (Utilities|Time|GetWorldDeltaSeconds)) (Variables|MoveRate|GetmoveMulitplier)) false true))

(event Input|AxisEvents|InputAxisMouseYaw
  (params (AxisValue :type Float%20%28single-precision%29))
  ;[1 0.6032 0] Mouse Yaw Input
  (Pawn|Input|AddControllerYawInput (* AxisValue (Variables|MouseRate|GetyawRate))))

(event Input|AxisEvents|InputAxisMousePitch
  (params (AxisValue :type Float%20%28single-precision%29))
  ;[0 1 1] Mouse Pitch Input
  (Pawn|Input|AddControllerPitchInput (* AxisValue (Variables|MouseRate|GetpitchRate))))

(event Input|AxisEvents|InputAxisKeyboardUp
  (params (AxisValue :type Float%20%28single-precision%29))
  ;[0 1 0.0718] Up/Down Input
  (if (not (Variables|Flags|GetgravityFlag))
    (Transformation|AddActorWorldOffset (Math|Vector|MakeVector 0.0 0.0 (* (* (.z (* (* (Transformation|GetActorUpVector) AxisValue) (Variables|MoveRate|GetvertRate))) (Utilities|Time|GetWorldDeltaSeconds)) (Variables|MoveRate|GetmoveMulitplier))) false true)))

(event Input|MouseEvents|MouseWheelAxis
  (params (AxisValue :type Float%20%28single-precision%29))
  ;[1 0 0.3135] Mouse Wheel - Change Movement Speed
  (CallFunction|ScrollMoveMultiplier AxisValue))

(event Input|KeyboardEvents|G
  (params (Key :type Key%20Structure :default "AnyKey"))
  ;[0 1 0.1057] Enabled/Disable gravity and collision
  (:Pressed
    (CallFunction|ToggleGravity)))

(event Input|KeyboardEvents|T
  (params (Key :type Key%20Structure :default "AnyKey"))
  ;[1 0.2357 0] Respawn the player
  (:Pressed
    (CallFunction|RespawnPlayer)))

(event Input|KeyboardEvents|P
  (params (Key :type Key%20Structure :default "AnyKey"))
  ;[0 1 0.3739] P Key - Toggle positional info
  (:Pressed
    (CallFunction|TogglePos)))

(event Input|KeyboardEvents|X
  (params (Key :type Key%20Structure :default "AnyKey"))
  ;[0 0.2016 1] Toggle info UI
  (:Pressed
    (CallFunction|ToggleInfo)))

(event Input|KeyboardEvents|I
  (params (Key :type Key%20Structure :default "AnyKey"))
  ;[0.7009 1 0] I Key - Toggle trace info
  (:Pressed
    (CallFunction|ToggleTrace)))

(fn ConstructionScript)

(fn GetForwardVector
  (return (Math|Vector|GetForwardVector (Math|Rotator|MakeRotator 0.0 0.0 (.yaw (Pawn|GetControlRotation :!class /Script/Engine.Pawn))))))

(fn GetRightVector
  (return (Math|Vector|GetRightVector (Math|Rotator|MakeRotator 0.0 0.0 (.yaw (Pawn|GetControlRotation :!class /Script/Engine.Pawn))))))

(fn ToggleGravity
  (bind _hud_info (Variables|UMG|GetHUD_Info))
  (bind _textgrav (Variables|/Game/Blueprints/Luffy_Dev/HUD_Debugger.HUD_Debugger_C|GettextGrav _hud_info))
  (bind _output_get (Variables|Flags|SetgravityFlag (not (Variables|Flags|GetgravityFlag))))
  (if _output_get
    (Variables|/Script/Engine.CharacterMovementComponent|SetGravityScale (Variables|Character|GetCharacterMovement) 1.0)
    (Collision|SetCollisionProfileName (Variables|Collision|GetCapsuleComponent) "Pawn" :!class /Script/Engine.PrimitiveComponent)
    (Physics|SetEnableGravity (Variables|Collision|GetCapsuleComponent) true)
    (Physics|SetSimulatePhysics (Variables|Collision|GetCapsuleComponent) true)
    (Rendering|Components|TextRender|SetText _textgrav "Gravity: On")
    (else
      (Variables|/Script/Engine.CharacterMovementComponent|SetGravityScale (Variables|Character|GetCharacterMovement) 0.0)
      (Collision|SetCollisionProfileName (Variables|Collision|GetCapsuleComponent) "NoCollision" :!class /Script/Engine.PrimitiveComponent)
      (Physics|SetEnableGravity (Variables|Collision|GetCapsuleComponent) false)
      (Physics|SetSimulatePhysics (Variables|Collision|GetCapsuleComponent) false)
      (Rendering|Components|TextRender|SetText _textgrav "Gravity: Off"))))

(fn RespawnPlayer
  (bind _spawnedvector (Variables|respawn|GetspawnedVector))
  (Class|GameplayStatics|SetWorldOriginLocation (Class|KismetMathLibrary|FTruncVector _spawnedvector))
  (Transformation|SetActorLocation _spawnedvector false true)
  (Development|PrintString "Position Reset" true true "(R=0.060636,G=1.000000,B=0.000000,A=1.000000)" 5.0))

(fn ToggleInfo
  (if (Variables|Flags|GetinfoFlag)
    (Widget|SetVisibility (Variables|/Game/Blueprints/Luffy_Dev/HUD_Debugger.HUD_Debugger_C|GetTextInfo (Variables|UMG|GetHUD_Info)) "Hidden")
    (Variables|Flags|SetinfoFlag false)
    (else
      (Widget|SetVisibility (Variables|/Game/Blueprints/Luffy_Dev/HUD_Debugger.HUD_Debugger_C|GetTextInfo (Variables|UMG|GetHUD_Info)) "Visible")
      (Variables|Flags|SetinfoFlag true))))

(fn ScrollMoveMultiplier
  (params (axisValue :type Float%20%28single-precision%29))
  (bind _output_get (LocalVariables|Set_localAxis axisValue))
  (if (!= _output_get 0.0)
    (if (> (LocalVariables|Get_localAxis) 0.0)
      (bind _output_get_2 (Variables|MoveRate|SetmoveMulitplier (Math|Float|Clamp(Float) (+ (Variables|MoveRate|GetmoveMulitplier) (* (Variables|MouseRate|GetmultiplierRate) (LocalVariables|Get_localAxis))) 0.01 1e+04)))
      (Rendering|Components|TextRender|SetText (Variables|/Game/Blueprints/Luffy_Dev/HUD_Debugger.HUD_Debugger_C|GettextSpeed (Variables|UMG|GetHUD_Info)) (Utilities|Text|ToText(String) (Utilities|String|Append (Utilities|String|ToString(Integer) (Math|Float|Floor (* _output_get_2 1e+02))) "% " "Speed")))
      (else
        (bind _output_get_3 (Variables|MoveRate|SetmoveMulitplier (Math|Float|Clamp(Float) (+ (Variables|MoveRate|GetmoveMulitplier) (* (Variables|MouseRate|GetmultiplierRate) (LocalVariables|Get_localAxis))) 0.01 2.0)))
        (Rendering|Components|TextRender|SetText (Variables|/Game/Blueprints/Luffy_Dev/HUD_Debugger.HUD_Debugger_C|GettextSpeed (Variables|UMG|GetHUD_Info)) (Utilities|Text|ToText(String) (Utilities|String|Append (Utilities|String|ToString(Integer) (Math|Float|Floor (* _output_get_3 1e+02))) "% " "Speed")))))))

(fn TogglePos
  (if (Variables|Flags|GetposFlag)
    (Widget|SetVisibility (Variables|/Game/Blueprints/Luffy_Dev/HUD_Debugger.HUD_Debugger_C|GettextPOS (Variables|UMG|GetHUD_Info)) "Hidden")
    (Widget|SetVisibility (Variables|/Game/Blueprints/Luffy_Dev/HUD_Debugger.HUD_Debugger_C|GettextRotation (Variables|UMG|GetHUD_Info)) "Hidden")
    (Variables|Flags|SetposFlag false)
    (else
      (Widget|SetVisibility (Variables|/Game/Blueprints/Luffy_Dev/HUD_Debugger.HUD_Debugger_C|GettextPOS (Variables|UMG|GetHUD_Info)) "Visible")
      (Widget|SetVisibility (Variables|/Game/Blueprints/Luffy_Dev/HUD_Debugger.HUD_Debugger_C|GettextRotation (Variables|UMG|GetHUD_Info)) "Visible")
      (Variables|Flags|SetposFlag true))))

(fn SetNewPosInfo
  (bind _returnvalue (Transformation|GetActorLocation))
  (bind _returnvalue_2 (Pawn|GetController))
  (bind _returnvalue_3 (Pawn|GetControlRotation _returnvalue_2 :!class /Script/Engine.Controller))
  (bind _output_get (LocalVariables|Set_localPOS (Utilities|String|Append " X: " (Utilities|String|ToString(Integer) (Math|Float|Floor (.x _returnvalue))) ", Y: " (Utilities|String|ToString(Integer) (Math|Float|Floor (.y _returnvalue))) ", Z: " (Utilities|String|ToString(Integer) (Math|Float|Floor (.z _returnvalue))) " ")))
  (Rendering|Components|TextRender|SetText (Variables|/Game/Blueprints/Luffy_Dev/HUD_Debugger.HUD_Debugger_C|GettextPOS (Variables|UMG|GetHUD_Info)) (Utilities|Text|ToText(String) _output_get))
  (Rendering|Components|TextRender|SetText (Variables|/Game/Blueprints/Luffy_Dev/HUD_Debugger.HUD_Debugger_C|GettextRotation (Variables|UMG|GetHUD_Info)) (Utilities|Text|ToText(String) (Utilities|String|Append " Y: " (Utilities|String|ToString(Integer) (Math|Float|Floor (.yaw _returnvalue_3))) ", P: " (Utilities|String|ToString(Integer) (Math|Float|Floor (.pitch _returnvalue_3))) ", R: " (Utilities|String|ToString(Integer) (Math|Float|Floor (.roll _returnvalue_3))) " "))))

(fn ToggleTrace
  (if (Variables|Flags|GettraceFlag)
    (Widget|SetVisibility (Variables|/Game/Blueprints/Luffy_Dev/HUD_Debugger.HUD_Debugger_C|GettextTrace (Variables|UMG|GetHUD_Info)) "Hidden")
    (Variables|Flags|SettraceFlag false)
    (else
      (Widget|SetVisibility (Variables|/Game/Blueprints/Luffy_Dev/HUD_Debugger.HUD_Debugger_C|GettextTrace (Variables|UMG|GetHUD_Info)) "Visible")
      (Variables|Flags|SettraceFlag true))))

(fn TracetoObject
  (bind _returnvalue (Game|GetPlayerCameraManager 0))
  (bind _returnvalue_2 (Transformation|GetActorLocation _returnvalue))
  (bind (_outhit _returnvalue_3) (Collision|LineTraceForObjects _returnvalue_2 (+ (* (Transformation|GetActorForwardVector _returnvalue) (Variables|Trace|GettraceDistance)) _returnvalue_2) (LocalVariables|Get_objectTypes) false 0 "None" true "(R=1.000000,G=0.000000,B=0.000000,A=1.000000)" "(R=0.000000,G=1.000000,B=0.000000,A=1.000000)" 1e+01))
  (if _returnvalue_3
    (Rendering|Components|TextRender|SetText (Variables|/Game/Blueprints/Luffy_Dev/HUD_Debugger.HUD_Debugger_C|GettextTrace (Variables|UMG|GetHUD_Info)) (Utilities|Text|ToText(String) (Utilities|GetDisplayName (.HitActor (Collision|BreakHitResult _outhit)))))
    (else
      (Rendering|Components|TextRender|SetText (Variables|/Game/Blueprints/Luffy_Dev/HUD_Debugger.HUD_Debugger_C|GettextTrace (Variables|UMG|GetHUD_Info)) "No object"))))